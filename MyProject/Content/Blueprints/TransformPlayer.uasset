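; TransformPlayer is a one-shot trigger actor that switches the player to another pawn.
; When its TriggerArea is overlapped, a helper checks that the actor is a BoxTumbleController pawn with IsSphere set.
; On a match, it advances PawnIndex with wraparound through PawnArray, makes player controller 0 possess that pawn, then destroys both the overlapping pawn and itself.
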(event OnComponentBeginOverlap(TriggerArea)
  (params (OtherActor :type Actor%20Object%20Reference) (OtherComp :type Primitive%20Component%20Object%20Reference) (OtherBodyIndex :type Integer) (bFromSweep :type Boolean) (SweepResult :type Hit%20Result%20Structure%20%28by%20ref%29))
  (bind _issphere (CallFunction|HasIsCircleBoost OtherActor))
  (if _issphere
    (Variables|Default|SetPawn%20Index (Math|Integer|%(Integer) (+ (Variables|Default|GetPawn%20Index) 1) (Utilities|Array|Length (Variables|Default|GetPawn%20Array))))
    (Pawn|Possess (Game|GetPlayerController 0) (Utilities|Array|Get(acopy) (Variables|Default|GetPawn%20Array) (Variables|Default|GetPawn%20Index)))
    (Actor|DestroyActor OtherActor)
    (Actor|DestroyActor)))

(fn ConstructionScript)

(fn HasIsCircleBoost
  (params (otherActor :type Actor%20Object%20Reference))
  (bind _aspawn (Utilities|Casting|CastToPawn otherActor)
    (:then
      (bind _asboxtumblecontroller_c (Utilities|Casting|CastToBoxTumbleController _aspawn)
        (:then
          (LocalVariables|Setvictory (Variables|/Game/Blueprints/BoxTumbleController.BoxTumbleController_C|GetisSphere _asboxtumblecontroller_c)))
        (:CastFailed
          (LocalVariables|Setvictory false :!label _label))))
    (:CastFailed
      (goto _label)))
  (return (LocalVariables|Getvictory)))