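; GravChangeVolume is an overlap volume that replaces normal gravity with its own Gravity vector for actors inside it.
; Entering actors have gravity disabled on their primitive components, and exiting restores it.
; Each tick it applies Gravity to those components as a velocity-change impulse, unscaled by delta time.
; It also aligns an overlapping BoxTumbleController's GravityRotator against that vector, resetting it to zero on exit.
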(event `self.ReceiveActorEndOverlap`
  (params (OtherActor :type "Actor Object Reference"))
  ;[1 1 1] Enable Gravity on Exit
  (bind _asboxtumblecontroller_c (cast `/Game/Blueprints/BoxTumbleController` OtherActor)
    (:`then`
      (set `/Game/Blueprints/BoxTumbleController.GravityRotator` (`KismetMathLibrary.MakeRot` 0.0) _asboxtumblecontroller_c))
    (:`CastFailed`
      _))
  (for _array_element (`self.K2_GetComponentsByClass` OtherActor "/Script/Engine.PrimitiveComponent")
    (bind _asprimitivecomponent (cast `PrimitiveComponent` _array_element))
    (`PrimitiveComponent.SetEnableGravity` _asprimitivecomponent true)))

(event `self.ReceiveActorBeginOverlap`
  (params (OtherActor :type "Actor Object Reference"))
  ;[1 1 1] Disable Gravity on Overlap
  (for _array_element (`self.K2_GetComponentsByClass` OtherActor "/Script/Engine.PrimitiveComponent")
    (bind _asprimitivecomponent (cast `PrimitiveComponent` _array_element))
    (`PrimitiveComponent.SetEnableGravity` _asprimitivecomponent false)))

(event `self.ReceiveTick`
  (params (DeltaSeconds :type "Float (single-precision)"))
  (for _array_element (`self.GetOverlappingActors` "/Script/Engine.Actor")
    (bind _asboxtumblecontroller_c (cast `/Game/Blueprints/BoxTumbleController` _array_element)
      (:`then`
        (set `/Game/Blueprints/BoxTumbleController.GravityRotator` (`KismetMathLibrary.MakeRotFromZ` (`KismetMathLibrary.NegateVector` (`self.Gravity`))) _asboxtumblecontroller_c))
      (:`CastFailed`
        _))
    (for _array_element_2 (`self.K2_GetComponentsByClass` _array_element "/Script/Engine.PrimitiveComponent")
      (bind _asprimitivecomponent (cast `PrimitiveComponent` _array_element_2))
      (`PrimitiveComponent.AddImpulse` _asprimitivecomponent (`self.Gravity`) "None" true))))

(fn `UserConstructionScript`)