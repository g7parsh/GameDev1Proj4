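; Player ball Blueprint that rolls by camera-relative torque and gains abilities from tagged powerups.
; Hit events re-arm jumping and pass actor tags to UpdateFlags, which unlocks jump, super jump, boost, sphere or climb before pickups are destroyed.
; Tick charges held super jump on a cubic curve and boost on a square-root curve, released as impulses, with a boost cooldown.
; Mouse input orbits the spring arm with clamped pitch.
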(event EventHit
  (params (MyComp :type Primitive%20Component%20Object%20Reference) (Other :type Actor%20Object%20Reference) (OtherComp :type Primitive%20Component%20Object%20Reference) (bSelfMoved :type Boolean) (HitLocation :type Vector :default "0, 0, 0") (HitNormal :type Vector :default "0, 0, 0") (NormalImpulse :type Vector :default "0, 0, 0") (Hit :type Hit%20Result%20Structure%20%28by%20ref%29))
  ;[1 1 1] OnCollide
  (Variables|Default|SethasLanded true)
  (bind _shoulddestroyobject (CallFunction|UpdateFlags (Variables|/Script/Engine.Actor|GetTags Other)))
  (if _shoulddestroyobject
    (Actor|DestroyActor Other)
    (Components|Activation|Activate (Variables|Default|GetPowerupParticles) false)))

(event EventTick
  (params (DeltaSeconds :type Float%20%28single-precision%29))
  ;[1 1 1] Update
  (CallFunction|ChargeSuperJump DeltaSeconds)
  (CallFunction|ChargeBoost DeltaSeconds)
  (Variables|Default|SetboostCooldown (+ DeltaSeconds (Variables|Default|GetboostCooldown)))
  (if (and (> (Variables|Default|GetboostCooldown) 1.0) (not (Variables|Default|GetcanBoost)))
    (Variables|Default|SetboostCooldown 0.0)
    (Variables|Default|SetcanBoost true)))

(event Input|ActionEvents|InputActionJump
  (bind _initialjumpimpulse (Variables|Default|GetinitialJumpImpulse))
  (bind _jumpcharge (Variables|Default|GetjumpCharge))
  ;[1 1 1] OnJump
  (:Pressed
    (if (and (Variables|Default|GethasSuperJumpPowerup) (Variables|Default|GethasLanded))
      (Components|Activation|Activate _jumpcharge false)
      (Variables|Default|SetsuperJumpIsCharging true)
      (Variables|Default|SetSuperJumpCharge _initialjumpimpulse)
      (elif (and (Variables|Default|GethasLanded) (Variables|Default|GethasJumpPowerup))
        (Physics|AddImpulse (Variables|Default|GetBall) (Math|Vector|MakeVector 0.0 0.0 (Variables|Default|GetJumpImpulse)) "None" true :!label _label)
        (Variables|Default|SethasLanded false)
        (Variables|Default|SetJumpImpulse _initialjumpimpulse))))
  (:Released
    (if (and (Variables|Default|GethasSuperJumpPowerup) (Variables|Default|GethasLanded))
      (Components|Activation|Deactivate _jumpcharge)
      (Variables|Default|SetsuperJumpIsCharging false)
      (Variables|Default|SetJumpImpulse (Variables|Default|GetSuperJumpCharge))
      (Variables|Default|SetTimeSinceLastJumpCharge 0.0)
      (goto _label))))

(event Input|AxisEvents|InputAxisMoveForward
  (params (AxisValue :type Float%20%28single-precision%29))
  ;[1 1 1] Roll forwards/backwards
  (Class|PrimitiveComponent|AddTorque (Variables|Default|GetBall) (* (Math|Vector|GetRightVector (Class|KismetMathLibrary|MakeRot 0.0 (Variables|Default|GetCamYaw) 0.0)) (* AxisValue (Variables|Default|GetRollTorque))) "None"))

(event Input|AxisEvents|InputAxisMoveRight
  (params (AxisValue :type Float%20%28single-precision%29))
  ;[1 1 1] Roll left/right
  (Class|PrimitiveComponent|AddTorque (Variables|Default|GetBall) (Math|Vector|NegateVector (* (Math|Vector|GetForwardVector (Class|KismetMathLibrary|MakeRot 0.0 (Variables|Default|GetCamYaw) 0.0)) (* AxisValue (Variables|Default|GetRollTorque)))) "None"))

(event Input|MouseEvents|MouseX
  (params (AxisValue :type Float%20%28single-precision%29))
  ;[1 1 1] Camera
  (bind (_newyaw _newpitch) (CallFunction|CameraRotation AxisValue (Class|Actor|GetInputAxisKeyValue) (Variables|Default|GetCamYaw) (Variables|Default|GetCamPitch)))
  (Variables|Default|SetCamYaw _newyaw)
  (Variables|Default|SetCamPitch _newpitch)
  (Components|MoveComponentTo (Variables|Default|GetSpringArm) "0, 0, 0" (Class|KismetMathLibrary|MakeRot _newpitch _newyaw 0.0) false false 0.2))

(event Input|KeyboardEvents|LeftShift
  (bind _hasboostpowerup (Variables|Default|GethasBoostPowerup))
  ;[1 1 1] Boost
  (:Pressed
    (if (and (Variables|Default|GetcanBoost) _hasboostpowerup)
      (Variables|Default|SetBoostIsCharging true)
      (Variables|Default|SetboostCharge (Variables|Default|GetinitialBoostAmount) :!label _label)
      (Variables|Default|SetcanBoost false)))
  (:Released
    (if (and _hasboostpowerup (Variables|Default|GetBoostIsCharging))
      (Components|Activation|Activate (Variables|Default|Getboosting) false)
      (Variables|Default|SetBoostIsCharging false)
      (Variables|Default|SetboostDeltaTime 0.0)
      (if (Variables|Default|GethasLanded)
        (Physics|AddImpulse (Variables|Default|GetBall) (* (Math|Vector|GetForwardVector (Class|KismetMathLibrary|MakeRot 0.0 (Variables|Default|GetCamYaw) 0.0)) (Variables|Default|GetboostCharge)) "None" true)
        (goto _label)))))

(fn ConstructionScript)

(fn ChargeSuperJump
  (params (deltaTime :type Float%20%28single-precision%29))
  ;[1 1 1] Charge Super Jump
  (if (Variables|Default|GetsuperJumpIsCharging)
    (Variables|Default|SetTimeSinceLastJumpCharge (+ deltaTime (Variables|Default|GetTimeSinceLastJumpCharge)))
    (if (>= 1.0 (Variables|Default|GetTimeSinceLastJumpCharge))
      (Variables|Default|SetSuperJumpCharge (* (Variables|Default|GetinitialJumpImpulse) (+ 1.0 (* 2.0 (Math|Float|Power (Variables|Default|GetTimeSinceLastJumpCharge) 3.0))))))))

(fn UpdateFlags
  (params (tags :type Array%20of%20Names))
  ;[1 1 1] UpdateFlags
  (if (Utilities|Array|ContainsItem tags (Utilities|String|StringToName "Jump"))
    (Variables|Default|SethasJumpPowerup true)
    (LocalVariables|SetdestroyObject true))
  (if (Utilities|Array|ContainsItem tags (Utilities|String|StringToName "SuperJump"))
    (Variables|Default|SethasSuperJumpPowerup true)
    (LocalVariables|SetdestroyObject true))
  (if (Utilities|Array|ContainsItem tags (Utilities|String|StringToName "Boost"))
    (Variables|Default|SethasBoostPowerup true)
    (LocalVariables|SetdestroyObject true))
  (if (Utilities|Array|ContainsItem tags (Utilities|String|StringToName "Sphere"))
    (Variables|Default|SetisSphere true)
    (LocalVariables|SetdestroyObject true))
  (if (Utilities|Array|ContainsItem tags (Utilities|String|StringToName "Climb"))
    (Variables|Default|SethasClimbingPowerup true)
    (LocalVariables|SetdestroyObject true))
  (return (LocalVariables|GetdestroyObject)))

(fn ChargeBoost
  (params (time :type Float%20%28single-precision%29))
  ;[1 1 1] Update
  (if (Variables|Default|GetBoostIsCharging)
    (Variables|Default|SetboostDeltaTime (+ time (Variables|Default|GetboostDeltaTime)))
    (if (>= 1.0 (Variables|Default|GetboostDeltaTime))
      (Variables|Default|SetboostCharge (* (Math|Float|Power (Variables|Default|GetboostDeltaTime) 0.5) (Variables|Default|GetinitialBoostAmount))))))

(fn CameraRotation
  (params (MouseX :type Float%20%28single-precision%29) (MouseY :type Float%20%28single-precision%29) (CamYaw :type Float%20%28single-precision%29) (CamPitch :type Float%20%28single-precision%29))
  ;[1 1 1] Camera Rotation
  (return (Math|Float|%(Float) (+ (* (Variables|Default|GetCamYawSpeed) MouseX) CamYaw) 3.6e+02) (Math|Float|ClampAngle (+ CamPitch (* MouseY (Variables|Default|GetCamPitchSpeed))) -7e+01 -1e+01)))