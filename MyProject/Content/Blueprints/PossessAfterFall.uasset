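; PossessAfterFall is a one-shot trigger that hands player control to a BoxTumbleController pawn when any actor overlaps it.
; It possesses the pawn referenced by ToPosess and makes it the view target, then destroys the overlapping actor, the referenced Camera and itself.
; A helper, ObjectHasCircle, reads HasClimbingPowerup through chained casts but is not called by the overlap logic.
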(event EventActorBeginOverlap
  (params (OtherActor :type Actor%20Object%20Reference))
  (bind _returnvalue (Game|GetPlayerController 0))
  (bind _asboxtumblecontroller_c (Utilities|Casting|CastToBoxTumbleController (Variables|Default|GettoPosess)))
  (Pawn|Possess _returnvalue _asboxtumblecontroller_c)
  (Game|Player|SetViewTargetwithBlend _returnvalue _asboxtumblecontroller_c 0.0 "VTBlend_Linear" 0.0 false)
  (Actor|DestroyActor OtherActor)
  (Actor|DestroyActor (Variables|Default|GetCamera))
  (Actor|DestroyActor))

(fn ConstructionScript)

(fn ObjectHasCircle
  (params (NewParam :type Actor%20Object%20Reference))
  (bind _aspawnactionscomponent (Utilities|Casting|CastToPawnActionsComponent NewParam)
    (:then
      (bind _asboxtumblecontroller_c (Utilities|Casting|CastToBoxTumbleController _aspawnactionscomponent)
        (:then
          (LocalVariables|Setvictory (Variables|/Game/Blueprints/BoxTumbleController.BoxTumbleController_C|GethasClimbingPowerup _asboxtumblecontroller_c))
          (return (LocalVariables|Getvictory)))
        (:CastFailed
          _)))
    (:CastFailed
      _))
  (LocalVariables|Setvictory false))