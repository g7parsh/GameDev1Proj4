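; Player-controlled physics box pawn that tumbles around with mouse-driven camera and a forward boost, toggling box visibility on possess and unpossess.
; Mouse input feeds CameraRotation, which wraps yaw and clamps pitch to rotate the camera arm.
; Movement input applies camera-yaw-relative torque plus velocity-change impulses, gated by CanMove and an angular velocity cap.
; Boost adds a camera-forward impulse, then waits on a short delay-based cooldown.
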(event `self.ReceiveUnpossessed`
  (params (OldController :type "Controller Object Reference"))
  (`SceneComponent.ToggleVisibility` (`self.Box`) false :!label _label))

(event `self.ReceivePossessed`
  (params (NewController :type "Controller Object Reference"))
  (goto _label))

(event `InputAxisKey|MouseX`
  (params (AxisValue :type "Float (single-precision)"))
  ;[1 1 1] Camera
  (bind (_updatedyaw _updatedpitch) (`self.CameraRotation` AxisValue (stale `InputAxisKey|MouseY` AxisValue) (`self.CamYaw`) (`self.CamPitch`)))
  (set `self.CamPitch` _updatedpitch)
  (set `self.CamYaw` _updatedyaw)
  (`KismetSystemLibrary.MoveComponentTo` (`self.CameraArm`) (0.0 0.0 0.0) (`KismetMathLibrary.MakeRot` _updatedpitch _updatedyaw)))

(event `InputAxisKey|MouseY`
  (params (AxisValue :type "Float (single-precision)"))
  ;[1 1 1] Camera
)

(event `InputAxis|MoveForward`
  (params (AxisValue :type "Float (single-precision)"))
  (bind _box (`self.Box`))
  (bind _returnvalue (`KismetMathLibrary.MakeRot` 0.0 (`self.CamYaw`)))
  ;[1 1 1] Move Forward
  (bind _returnvalue_2 (`PrimitiveComponent.GetPhysicsAngularVelocity` (`self.Box`) "None"))
  (if (and (`self.CanMove`) (< (`KismetMathLibrary.VSize` _returnvalue_2) (`self.AngularVelocityCap`)))
    (`PrimitiveComponent.AddTorque` _box (* (`KismetMathLibrary.GetRightVector` _returnvalue) (* AxisValue (`self.RollTorque`))) "None")
    (`PrimitiveComponent.AddImpulse` _box (* (`KismetMathLibrary.GetForwardVector` _returnvalue) (* AxisValue (`self.RollSpeed`))) "None" true)))

(event `InputAxis|MoveRight`
  (params (AxisValue :type "Float (single-precision)"))
  (bind _box (`self.Box`))
  (bind _returnvalue (`KismetMathLibrary.MakeRot` 0.0 (`self.CamYaw`)))
  ;[1 1 1] Move Sideways
  (bind _returnvalue_2 (`PrimitiveComponent.GetPhysicsAngularVelocity` (`self.Box`) "None"))
  (if (and (`self.CanMove`) (< (`KismetMathLibrary.VSize` _returnvalue_2) (`self.AngularVelocityCap`)))
    (`PrimitiveComponent.AddTorque` _box (`KismetMathLibrary.NegateVector` (* (`KismetMathLibrary.GetForwardVector` _returnvalue) (* AxisValue (`self.RollTorque`)))) "None")
    (`PrimitiveComponent.AddImpulse` _box (* (`KismetMathLibrary.GetRightVector` _returnvalue) (* AxisValue (`self.RollSpeed`))) "None" true)))

(event `InputAction|Boost`
  (:`Pressed`
    (if (`self.BoostReady`)
      (`PrimitiveComponent.AddImpulse` (`self.Box`) (* (`KismetMathLibrary.GetForwardVector` (`KismetMathLibrary.MakeRot` 0.0 (`self.CamYaw`))) (`self.BoostSpeed`)) "None" false)
      (set `self.BoostReady` false)
      (`KismetSystemLibrary.Delay` 2.0)
      (set `self.BoostReady` true))))

(fn `CameraRotation`
  (params (MouseX :type "Float (double-precision)") (MouseY :type "Float (double-precision)") (CurrentYaw :type "Float (double-precision)") (CurrentPitch :type "Float (double-precision)"))
  (returns (UpdatedYaw :type "Float (double-precision)") (UpdatedPitch :type "Float (double-precision)"))
  ;[1 1 1] Camera Rotation
  (return (mod (+ (* (`self.CamYawSpeed`) MouseX) CurrentYaw) 360.0) (`KismetMathLibrary.ClampAngle` (+ CurrentPitch (* MouseY (`self.CamPitchSpeed`))) -70.0 -10.0)))

(fn `UserConstructionScript`)